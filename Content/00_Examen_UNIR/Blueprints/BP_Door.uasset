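; BP_Door is a two-panel sliding door actor that other code opens or closes.
; OpenCloseDoor takes a boolean and calls either the OpenDoor or CloseDoor event.
; OpenDoor plays a Timeline that lerps the NegDoor and PosDoor relative locations apart in opposite X directions, teleporting without sweep.
; CloseDoor reverses the same Timeline to slide the panels back together.
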(event `OpenDoor`
  (bind (_direction _value) (`Timeline|Timeline` :!label _label)
    (:`Update`
      (`SceneComponent.K2_SetRelativeLocation` (`self.NegDoor`) (`KismetMathLibrary.VLerp` (0.0 0.0 0.0) (-150.0 0.0 0.0) _value) false true)
      (`SceneComponent.K2_SetRelativeLocation` (`self.PosDoor`) (`KismetMathLibrary.VLerp` (0.0 0.0 0.0) (150.0 0.0 0.0) _value) false true))))

(event `CloseDoor`
  (goto _label :!via `Reverse`))

(fn `OpenCloseDoor`
  (params (isOpen :type Boolean))
  (if isOpen
    (`self.OpenDoor`)
    (else
      (`self.CloseDoor`))))

(fn `UserConstructionScript`)