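; BP_FloorButton is a floor switch that opens and closes a linked Door when the player has enough keys.
; Its Box overlap sends itself to the actor through InteractDoorMessage, and end overlap clears the top-down character's Switch reference.
; ToggleSwitch compares PlayerKeys with the Door's NeededKeys, then uses a FlipFlop to toggle the door and glyph color.
; With too few keys, it prints the missing count in Spanish.
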(event `self.Box.OnComponentBeginOverlap`
  (params (OverlappedComponent :type "PrimitiveComponent Object Reference") (OtherActor :type "Actor Object Reference") (OtherComp :type "PrimitiveComponent Object Reference") (OtherBodyIndex :type Integer) (bFromSweep :type Boolean) (SweepResult :type "HitResult Structure (by ref)"))
  (message `/Game/00_Examen_UNIR/Blueprints/I_Interactions.InteractDoor` OtherActor self))

(event `self.Box.OnComponentEndOverlap`
  (params (OverlappedComponent :type "PrimitiveComponent Object Reference") (OtherActor :type "Actor Object Reference") (OtherComp :type "PrimitiveComponent Object Reference") (OtherBodyIndex :type Integer))
  (bind _asbp_top_down_character (cast `/Game/TopDown/Blueprints/BP_TopDownCharacter` OtherActor))
  (set `/Game/TopDown/Blueprints/BP_TopDownCharacter.Switch` null _asbp_top_down_character))

(fn `ToggleSwitch`
  (params (PlayerKeys :type Integer))
  (bind _glyphs (`self.Glyphs`))
  (bind _ison (`self.IsOn`))
  (bind _neededkeys (`/Game/00_Examen_UNIR/Blueprints/BP_Door.NeededKeys` (`self.Door`)))
  (`KismetSystemLibrary.PrintString` "Hello")
  (if (>= PlayerKeys _neededkeys)
    (bind _isa (`/Engine/EditorBlueprintResources/StandardMacros.FlipFlop`)
      (:`A`
        (set `self.IsOn` true)
        (`PrimitiveComponent.SetMaterial` _glyphs 0 "/Game/00_Examen_UNIR/Materials/M_Accents_Green.M_Accents_Green")
        (`/Game/00_Examen_UNIR/Blueprints/BP_Door.OpenCloseDoor` (`self.Door`) _ison)
        (`KismetSystemLibrary.PrintString` (`KismetStringLibrary.Conv_BoolToString` _ison)))
      (:`B`
        (bind _output_get (set `self.IsOn` _isa))
        (`PrimitiveComponent.SetMaterial` _glyphs 0 "/Game/00_Examen_UNIR/Materials/M_Accents_White.M_Accents_White")
        (`/Game/00_Examen_UNIR/Blueprints/BP_Door.OpenCloseDoor` (`self.Door`) _output_get)
        (`KismetSystemLibrary.PrintString` (`KismetStringLibrary.Conv_BoolToString` _output_get))))
    (else
      (`KismetSystemLibrary.PrintString` (`KismetStringLibrary.Concat_StrStr` "Te faltan " (`KismetStringLibrary.Conv_IntToString` (- _neededkeys (`local.PlayerKeys`))) " llaves.")))))

(fn `UserConstructionScript`)